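; DCGameMode_BP is a game mode Blueprint whose active graphs do nothing, as BeginPlay and the construction script are both empty.
; A disconnected, never-executed chain holds UI setup that creates the in-game UI and start menu widgets and stores them on DCPlayerController.
; That chain also sets game-only input and passes the controlled pawn to UI_Render_BP as the new render mesh.
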(event `self.ReceiveBeginPlay`)

(fn `UserConstructionScript`)