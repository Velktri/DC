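; WeaponRender_BP is a preview actor that displays a weapon skeletal mesh alongside a SceneCaptureComponent2D, which is set to keep ticking while the game is paused.
; SetNewWeapon swaps the mesh and resets its location and root rotation, or clears it when the input is invalid.
; UpdatePivotandScale then uniformly scales the mesh to fit DesiredSize using its bounds and offsets it to center the bounds origin on the pivot.
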(event `self.ReceiveBeginPlay`
  (`ActorComponent.SetTickableWhenPaused` (`self.SceneCaptureComponent2D`) true))

(event `Update Pivot and Scale`
  (bind _rendermesh (`self.RenderMesh`))
  (set `self.CurrentMeshSize` (`.BoxExtent` (`KismetSystemLibrary.GetComponentBounds` (`self.RenderMesh`))))
  (`SceneComponent.SetWorldScale3D` (`self.RenderMesh`) (* (`SceneComponent.K2_GetComponentScale` (`self.RenderMesh`)) (`KismetMathLibrary.FMin` (/ (.x (`self.DesiredSize`)) (.x (`self.CurrentMeshSize`))) (/ (.y (`self.DesiredSize`)) (.y (`self.CurrentMeshSize`))) (/ (.z (`self.DesiredSize`)) (.z (`self.CurrentMeshSize`))))))
  (`SceneComponent.K2_AddLocalOffset` (`self.RenderMesh`) (- (`SceneComponent.K2_GetComponentLocation` _rendermesh) (`KismetSystemLibrary.GetComponentBounds` _rendermesh)) false false))

(fn `NewFunction_0`
  (params (InputObject :type "Object Object Reference") (InputPin :type "SkeletalMesh Object Reference"))
  (bind _rendermesh (`self.RenderMesh`))
  (`/Engine/EditorBlueprintResources/StandardMacros.IsValid` InputObject
    (:`Is Valid`
      (`SkinnedMeshComponent.SetSkinnedAssetAndUpdate` _rendermesh InputPin true)
      (`SceneComponent.K2_SetRelativeLocation` _rendermesh (0.0 0.0 0.0) false false)
      (`SceneComponent.K2_SetRelativeRotation` :`self` (`self.MeshRoot`)))
    (:`Is Not Valid`
      (`SkinnedMeshComponent.SetSkinnedAssetAndUpdate` _rendermesh null true))))

(fn `Set New Weapon`
  (params (InMesh :type "SkeletalMesh Object Reference"))
  (`self.NewFunction_0` InMesh InMesh)
  (`self.Update Pivot and Scale`))

(fn `UserConstructionScript`)