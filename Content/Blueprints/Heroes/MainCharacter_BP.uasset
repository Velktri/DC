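; MainCharacter_BP is a hero character Blueprint whose health drains steadily over time.
; Tick adds delta seconds to SecondCheck and, each time it reaches one second, carries over the remainder and subtracts a fixed amount from CurrentHealth.
; The graph has no clamp or death handling, and BeginPlay, overlap and the construction script are empty.
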(event `self.ReceiveTick`
  (params (DeltaSeconds :type "Float (single-precision)"))
  (bind _output_get (set `self.secondCheck` (+ DeltaSeconds (`self.secondCheck`))))
  (if (>= _output_get 1.0)
    (set `self.secondCheck` (- (`self.secondCheck`) 1.0))
    (set `self.CurrentHealth` (- (`self.CurrentHealth`) 3))))

(fn `UserConstructionScript`)