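; DCGameMode_BP is a game mode Blueprint that sets up the player's UI when play begins.
; On BeginPlay it creates the InGameUI widget and adds it to the viewport, then creates a StartMenu widget without displaying it, storing both on the DCPlayerController.
; It switches input to game only and passes the controlled pawn to the controller's UI_Render_BP weapon render reference via SetNewRenderMesh.
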(event `self.ReceiveBeginPlay`
  (bind _returnvalue (`|CreateWidget` "/Game/UI/InGameUI.InGameUI_C" (`GameplayStatics.GetPlayerController` 0)))
  (`UserWidget.AddToViewport` _returnvalue 0)
  (bind _asdcplayer_controller (cast `DCPlayerController` (`Widget.GetOwningPlayer` _returnvalue)))
  (set `DCPlayerController.InGameUI` _returnvalue _asdcplayer_controller)
  (bind _returnvalue_2 (`|CreateWidget` "/Game/UI/Menus/StartMenu.StartMenu_C" _asdcplayer_controller))
  (set `DCPlayerController.StartMenuWidget` _returnvalue_2 _asdcplayer_controller)
  (`WidgetBlueprintLibrary.SetInputMode_GameOnly` _asdcplayer_controller)
  (bind _asui_render_bp (cast `/Game/Blueprints/UI_Render_BP` (`DCPlayerController.WeaponRenderRef` _asdcplayer_controller)))
  (`UI_Render.SetNewRenderMesh` _asui_render_bp (`Controller.K2_GetPawn` _asdcplayer_controller)))

(fn `UserConstructionScript`)